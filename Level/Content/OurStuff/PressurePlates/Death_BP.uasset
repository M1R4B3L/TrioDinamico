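; Death_BP is an overlap-triggered death actor that respawns the first-person player character.
; On overlap it destroys the BP_FirstPersonCharacter, spawns a new one of the same class at SpawnTransform and has player controller 0 possess it.
; It then replaces each BP_Rifle1 in the level with a new one at SpawnTransform, calling TeleportPlayer on the new character inside that loop.
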(event Collision|EventActorBeginOverlap
  (params (OtherActor :type Actor%20Object%20Reference))
  (bind _spawn_transform (Variables|Default|GetSpawn%20Transform))
  (bind _asbp_first_person_character (Utilities|Casting|CastToBP_FirstPersonCharacter OtherActor))
  (bind _output_get (Variables|Default|SetPlayerBP _asbp_first_person_character))
  (Actor|DestroyActor (Variables|Default|GetPlayerBP))
  (bind _returnvalue (Game|SpawnActorfromClass (Utilities|GetClass _output_get) _spawn_transform "Undefined" 0 0))
  (Pawn|Possess (Game|GetPlayerController 0) _returnvalue)
  (bind _outactors (Actor|GetAllActorsOfClass "/Game/FirstPerson/Blueprints/BP_Rifle1.BP_Rifle1_C"))
  (for _array_element _outactors
    (Actor|DestroyActor _array_element)
    (Game|SpawnActorfromClass "/Game/FirstPerson/Blueprints/BP_Rifle1.BP_Rifle1_C" _spawn_transform "Undefined" 0 0)
    (Default|TeleportPlayer _returnvalue)))

(fn ConstructionScript)