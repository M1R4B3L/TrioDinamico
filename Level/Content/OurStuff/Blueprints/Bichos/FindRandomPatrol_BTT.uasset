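; Behavior tree task that picks a random patrol destination for a Melee_Char enemy.
; It sets the pawn's walk speed to PatrolSpeed, then searches for a random reachable point within PatrolRadius of its current location.
; The result goes to the PatrolLocation blackboard key, falling back to the pawn's own location if none is found.
; The task fails only when the pawn is not a Melee_Char.
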(event EventReceiveExecuteAI
  (params (OwnerController :type AI%20Controller%20Object%20Reference) (ControlledPawn :type Pawn%20Object%20Reference))
  (bind _returnvalue (Transformation|GetActorLocation ControlledPawn))
  (bind _patrol_radius (Variables|Default|GetPatrol%20Radius))
  (bind (_randomlocation _returnvalue_2) (AI|Navigation|GetRandomReachablePointinRadius _returnvalue _patrol_radius 0 0))
  (bind _asmelee_char (Utilities|Casting|CastToMelee_Char ControlledPawn)
    (:then
      (Default|UpdateWalkSpeed _asmelee_char (Variables|Default|GetPatrol%20Speed))
      (if _returnvalue_2
        (AI|BehaviorTree|SetBlackboardValueasVector (Variables|Default|GetPatrolLocation) _randomlocation)
        (else
          (AI|BehaviorTree|SetBlackboardValueasVector (Variables|Default|GetPatrolLocation) _returnvalue)))
      (AI|BehaviorTree|FinishExecute true))
    (:CastFailed
      (AI|BehaviorTree|FinishExecute false))))